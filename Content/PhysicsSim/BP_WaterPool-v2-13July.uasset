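; BP_WaterPool is a physics-sim water pool actor that turns its Niagara effect when a GrippableStaticMeshActor begins overlapping it.
; Each overlap event lerps the stored ReturnedRot slightly toward that actor's root rotation, using half the frame delta as alpha, and prints the result.
; The effect receives the lerped value as relative rotation and its own world location as relative location.
; Tick is empty, so rotation advances only on overlap begin.
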(event `self.ReceiveBeginPlay`)

(event `self.ReceiveActorBeginOverlap`
  (params (OtherActor :type "Actor Object Reference"))
  (bind _niagara (`self.Niagara`))
  (bind _asgrippable_static_mesh_actor (cast `GrippableStaticMeshActor` OtherActor))
  (bind _returnvalue (`KismetMathLibrary.RLerp` (`self.ReturnedRot`) (`SceneComponent.K2_GetComponentRotation` (`Actor.RootComponent` _asgrippable_static_mesh_actor)) (* (`GameplayStatics.GetWorldDeltaSeconds`) 0.5)))
  (`SceneComponent.K2_SetRelativeLocationAndRotation` _niagara (`SceneComponent.K2_GetComponentLocation` _niagara) _returnvalue false false)
  (bind _output_get (set `self.ReturnedRot` _returnvalue))
  (`KismetSystemLibrary.PrintString` (`KismetStringLibrary.Conv_RotatorToString` _output_get) true true (struct :`G` 0.66 :`B` 1.0 :`A` 1.0) 1.0))

(event `self.ReceiveTick`
  (params (DeltaSeconds :type "Float (single-precision)")))

(fn `UserConstructionScript`)